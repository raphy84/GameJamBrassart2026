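; Cannon scanner that detects monsters around a center point, feeds a cannon monitor and delivers frequency shots to targets.
; Each tick it sphere-traces, sums frequency and distance (as energy) of monsters between two yaw bounds for the monitor, and draws debug lines.
; A small sphere-trace hit kills the player.
; AimCanon sets angle and range; Shoot sends its frequency to hits inside that 45-degree sector and one of five distance bands.
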(event Custom|AimCanon
  (params (Angle :type Float%20%28double-precision%29) (Range :type Float%20%28double-precision%29))
  (Variables|Default|SetRange Range)
  (bind _output_get (Variables|Default|SetAngleC Angle))
  (Transformation|SetWorldRotation (Variables|Default|GetC) (Math|Rotator|MakeRotator 0.0 0.0 _output_get) false false))

(event Custom|Shoot
  (params (Frequence :type Float%20%28double-precision%29))
  (bind _anglec (Variables|Default|GetAngleC))
  (bind _outhits (Collision|MultiSphereTraceByChannel "0, 0, 0" "0, 0, 0" 3e+03 "TraceTypeQuery3" false 0 "ForOneFrame"))
  (for _array_element _outhits
    (if (and (<= (.yaw (Math|Rotator|FindLookatRotation (Variables|Default|GetCenter) (.ImpactPoint (Collision|BreakHitResult _array_element)))) (+ _anglec 45.0)) (>= (.yaw (Math|Rotator|FindLookatRotation (Variables|Default|GetCenter) (.ImpactPoint (Collision|BreakHitResult _array_element)))) _anglec))
      (switch int (Math|Float|Truncate (Variables|Default|GetRange))
        (:0
          (if (and (<= (Math|Vector|Distance(Vector) (.ImpactPoint (Collision|BreakHitResult _array_element)) (Variables|Default|GetCenter)) 3e+03) (>= (Math|Vector|Distance(Vector) (.ImpactPoint (Collision|BreakHitResult _array_element)) (Variables|Default|GetCenter)) 2.4e+03))
            (Class|BPIMonster|TryRun(Message) (.HitActor (Collision|BreakHitResult _array_element)) Frequence :!label _label)))
        (:1
          (if (and (<= (Math|Vector|Distance(Vector) (.ImpactPoint (Collision|BreakHitResult _array_element)) (Variables|Default|GetCenter)) 2.4e+03) (>= (Math|Vector|Distance(Vector) (.ImpactPoint (Collision|BreakHitResult _array_element)) (Variables|Default|GetCenter)) 1.8e+03))
            (goto _label)))
        (:2
          (if (and (<= (Math|Vector|Distance(Vector) (.ImpactPoint (Collision|BreakHitResult _array_element)) (Variables|Default|GetCenter)) 1.8e+03) (>= (Math|Vector|Distance(Vector) (.ImpactPoint (Collision|BreakHitResult _array_element)) (Variables|Default|GetCenter)) 1.2e+03))
            (goto _label)))
        (:3
          (if (and (<= (Math|Vector|Distance(Vector) (.ImpactPoint (Collision|BreakHitResult _array_element)) (Variables|Default|GetCenter)) 1.2e+03) (>= (Math|Vector|Distance(Vector) (.ImpactPoint (Collision|BreakHitResult _array_element)) (Variables|Default|GetCenter)) 6e+02))
            (goto _label)))
        (:4
          (if (and (<= (Math|Vector|Distance(Vector) (.ImpactPoint (Collision|BreakHitResult _array_element)) (Variables|Default|GetCenter)) 6e+02) (>= (Math|Vector|Distance(Vector) (.ImpactPoint (Collision|BreakHitResult _array_element)) (Variables|Default|GetCenter)) 1e+01))
            (goto _label)))))))

(event EventBeginPlay
  (bind _asbp_first_person_character (Utilities|Casting|CastToBP_FirstPersonCharacter (Game|Player|GetPlayerPawn 0)))
  (Variables|Default|SetPlayer _asbp_first_person_character))

(event EventTick
  (params (DeltaSeconds :type Float%20%28single-precision%29))
  (Transformation|SetWorldRotation (Variables|Default|GetB) (Math|Rotator|MakeRotator 0.0 0.0 (Variables|Default|GetBAngle)) false false)
  (Transformation|SetWorldRotation (Variables|Default|GetA) (Math|Rotator|MakeRotator 0.0 0.0 (Variables|Default|GetAAngle)) false false)
  (Collision|LineTraceByChannel "0, 0, 0" (* (Math|Vector|GetForwardVector (Variables|Default|GetC)) 3000) "TraceTypeQuery4" false 0 "ForOneFrame" true "(R=0.061393,G=1.000000,B=0.000000,A=1.000000)")
  (Collision|LineTraceByChannel "0, 0, 0" (* (Math|Vector|GetForwardVector (Variables|Default|GetD)) 3000) "TraceTypeQuery4" false 0 "ForOneFrame" true "(R=0.006315,G=1.000000,B=0.000000,A=1.000000)")
  (Collision|LineTraceByChannel "0, 0, 0" (* (Math|Vector|GetForwardVector (Variables|Default|GetA)) 3000) "TraceTypeQuery4" false 0 "ForOneFrame")
  (Collision|LineTraceByChannel "0, 0, 0" (* (Math|Vector|GetForwardVector (Variables|Default|GetB)) 3000) "TraceTypeQuery4" false 0 "ForOneFrame" true "(R=0.000000,G=0.208597,B=1.000000,A=1.000000)")
  (Utilities|FlowControl|Sequence
    (:then_0
      (bind _returnvalue (Collision|SphereTraceByChannel "0, 0, 0" "0, 0, 0" 1e+01 "TraceTypeQuery3" false 0 "None"))
      (if _returnvalue
        (Default|Death (Variables|Default|GetPlayer))))
    (:then_1
      (bind _outhits (Collision|MultiSphereTraceByChannel "0, 0, 0" "0, 0, 0" 3e+03 "TraceTypeQuery3" false 0 "ForOneFrame"))
      (Variables|Default|SetAddEnergie 0.0)
      (Variables|Default|SetAddFrequence 0.0)
      (for _array_element _outhits
        (if (and (<= (.yaw (Math|Rotator|FindLookatRotation (Variables|Default|GetCenter) (.ImpactPoint (Collision|BreakHitResult _array_element)))) (Variables|Default|GetAAngle)) (>= (.yaw (Math|Rotator|FindLookatRotation (Variables|Default|GetCenter) (.ImpactPoint (Collision|BreakHitResult _array_element)))) (Variables|Default|GetBAngle)))
          (Variables|Default|SetAddFrequence (+ (Variables|/Game/Game/Blueprints/IA/BP_Monster.BP_Monster_C|GetFrequenceSent (.AsBP%20Monster (Utilities|Casting|CastToBP_Monster (.HitActor (Collision|BreakHitResult _array_element))))) (Variables|Default|GetAddFrequence)))
          (Variables|Default|SetAddEnergie (+ (Math|Vector|Distance(Vector) (.ImpactPoint (Collision|BreakHitResult _array_element)) (Variables|Default|GetCenter)) (Variables|Default|GetAddEnergie)))
          (else
            (Default|InfoMonster (Variables|Default|GetCannonMonitor) 0.0 0.0))))
      (Default|InfoMonster (Variables|Default|GetCannonMonitor) (Variables|Default|GetAddFrequence) (Variables|Default|GetAddEnergie)))))

(fn ConstructionScript)