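; BP_CannonMonitor is an interactable cannon monitor that moves the player's camera to its screen to set scanner angles and show monster readings.
; Dragging either button runs a looping timer that turns mouse X into mutually clamped left/right angles, feeding the CanonView widget and Scaner.
; InfoMonster sends jittered frequency and remapped energy to MonsterView, switching between static and an energy-pitched radio signal sound.
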(event OnClicked(BoutonDroite)
  (params (TouchedComponent :type Primitive%20Component%20Object%20Reference) (ButtonPressed :type Key%20Structure :default "None"))
  (Variables|Default|SetLocationX (.LocationX (Game|Player|GetMousePosition (Game|GetPlayerController 0))))
  (bind _returnvalue (Utilities|Time|SetTimerbyEvent (delegate Custom|TickLeft) 0.001 true))
  (Variables|Default|SetUnset _returnvalue))

(event OnReleased()
  (params (TouchedComponent :type Primitive%20Component%20Object%20Reference) (ButtonReleased :type Key%20Structure :default "None"))
  (Utilities|Time|PauseTimerbyHandle (Variables|Default|GetUnset))
  (Variables|Default|SetRotationYRight (Variables|Default|GetGetRotationYRight))
  (Variables|Default|SetRotationYLeft (Variables|Default|GetGetRotationYLeft)))

(event OnReleased(BoutonGauche)
  (params (TouchedComponent :type Primitive%20Component%20Object%20Reference) (ButtonReleased :type Key%20Structure :default "None"))
  (Utilities|Time|PauseTimerbyHandle (Variables|Default|GetUnset))
  (Variables|Default|SetRotationYRight (Variables|Default|GetGetRotationYRight))
  (Variables|Default|SetRotationYLeft (Variables|Default|GetGetRotationYLeft)))

(event OnReleased(BoutonDroite)
  (params (TouchedComponent :type Primitive%20Component%20Object%20Reference) (ButtonReleased :type Key%20Structure :default "None"))
  (Utilities|Time|PauseTimerbyHandle (Variables|Default|GetUnset))
  (Variables|Default|SetRotationYRight (Variables|Default|GetGetRotationYRight))
  (Variables|Default|SetRotationYLeft (Variables|Default|GetGetRotationYLeft)))

(event OnClicked(BoutonGauche)
  (params (TouchedComponent :type Primitive%20Component%20Object%20Reference) (ButtonPressed :type Key%20Structure :default "None"))
  (Variables|Default|SetLocationX (.LocationX (Game|Player|GetMousePosition (Game|GetPlayerController 0))))
  (bind _returnvalue (Utilities|Time|SetTimerbyEvent (delegate Custom|Tick) 0.001 true))
  (Variables|Default|SetUnset _returnvalue))

(event Custom|TickLeft
  (bind _returnvalue (Game|GetPlayerController 0))
  (bind _rotationyleft (Variables|Default|GetRotationYLeft))
  (bind _getrotationyright (Variables|Default|GetGetRotationYRight))
  (bind _locationx (Variables|Default|GetLocationX))
  (bind _scaner (Variables|Default|GetScaner))
  (bind _locationx_2 (Game|Player|GetMousePosition _returnvalue))
  (bind _returnvalue_2 (- 1.8e+02 _getrotationyright))
  (bind _returnvalue_3 (- _locationx _locationx_2))
  (bind _returnvalue_4 (/ _returnvalue_3 3.0))
  (bind _returnvalue_5 (+ _rotationyleft _returnvalue_4))
  (bind _returnvalue_6 (Math|Float|NormalizetoRange _returnvalue_5 0.0 1.8e+02))
  (bind _returnvalue_7 (+ _returnvalue_5 _returnvalue_6))
  (bind _returnvalue_8 (Math|Float|Clamp(Float) _returnvalue_7 0.0 _returnvalue_2))
  (Transformation|SetWorldRotation (Variables|Default|GetBoutonDroite) (Math|Rotator|MakeRotator 0.0 _returnvalue_8 0.0) false false)
  (bind _output_get (Variables|Default|SetGetRotationYLeft _returnvalue_8))
  (Default|ChangeValue (Variables|Default|GetCanonView) (/ _output_get 1.8e+02) (/ (stale Custom|Tick _output_get) 1.8e+02))
  (Variables|/Game/Game/Blueprints/Cannon/BP_Scaner.BP_Scaner_C|SetBAngle _scaner (- (* (/ (stale Custom|Tick _output_get) 1.8e+02) 3.6e+02) 1.8e+02))
  (bind _result (Math|Float|NegateFloat (- (* (/ _output_get 1.8e+02) 3.6e+02) 1.8e+02))
    (:%20%20
      (Variables|/Game/Game/Blueprints/Cannon/BP_Scaner.BP_Scaner_C|SetAAngle _scaner _result))))

(event Custom|InfoMonster
  (params (Frequence :type Float%20%28double-precision%29) (Energie :type Float%20%28double-precision%29))
  (bind _returnvalue (Math|Float|MapRangeClamped Energie 3e+03 0.0 0.0 1e+05))
  (Default|Calcule (Variables|Default|GetMonsterView) (Math|Random|RandomIntegerinRange (Math|Float|Truncate (- Frequence 3e+01)) (Math|Float|Truncate (+ Frequence 3e+01))) (Math|Float|Truncate _returnvalue))
  (if (== _returnvalue 1e+05)
    (Utilities|IsValid (Variables|Default|GetSoundScanerDetectRef)
      (:Is%20Valid
        (Class|AudioComponent|SetPaused (Variables|Default|GetSoundScanerDetectRef) true))
      (:Is%20Not%20Valid
        _))
    (Utilities|IsValid (Variables|Default|GetSoundScanerNoneRef)
      (:Is%20Valid
        (Class|AudioComponent|SetPaused (Variables|Default|GetSoundScanerNoneRef) false))
      (:Is%20Not%20Valid
        _))
    (Utilities|FlowControl|DoOnce false
      (:Completed
        (bind _returnvalue_2 (Audio|SpawnSound2D "/Game/Game/SoundDesign/Gresillements_Cue.Gresillements_Cue" 0.5 0.3 0.0 0))
        (Variables|Default|SetSoundScanerNoneRef _returnvalue_2)))
    (else
      (Utilities|IsValid (Variables|Default|GetSoundScanerDetectRef)
        (:Is%20Valid
          (Class|AudioComponent|SetPaused (Variables|Default|GetSoundScanerDetectRef) false)
          (Audio|Components|Audio|SetPitchMultiplier (Variables|Default|GetSoundScanerDetectRef) (Math|Float|Lerp 0.3 2.0 (Math|Float|MapRangeClamped _returnvalue 0.0 1e+05 0.0 1.0)))
          (Class|AudioComponent|SetPaused (Variables|Default|GetSoundScanerNoneRef) true))
        (:Is%20Not%20Valid
          _))
      (Utilities|FlowControl|DoOnce false
        (:Completed
          (bind _returnvalue_3 (Audio|SpawnSound2D "/Game/Game/SoundDesign/SignalRadio_Cue.SignalRadio_Cue" 0.3 0.3 0.0 0))
          (Variables|Default|SetSoundScanerDetectRef _returnvalue_3))))))

(event Custom|Tick
  (bind _returnvalue (Game|GetPlayerController 0))
  (bind _locationx (Variables|Default|GetLocationX))
  (bind _rotationyright (Variables|Default|GetRotationYRight))
  (bind _getrotationyleft (Variables|Default|GetGetRotationYLeft))
  (bind _scaner (Variables|Default|GetScaner))
  (bind _locationx_2 (Game|Player|GetMousePosition _returnvalue))
  (bind _returnvalue_2 (- 1.8e+02 _getrotationyleft))
  (bind _returnvalue_3 (- _locationx _locationx_2))
  (bind _returnvalue_4 (/ _returnvalue_3 3.0))
  (bind _returnvalue_5 (+ _rotationyright _returnvalue_4))
  (bind _returnvalue_6 (Math|Float|NormalizetoRange _returnvalue_5 0.0 1.8e+02))
  (bind _returnvalue_7 (+ _returnvalue_5 _returnvalue_6))
  (bind _returnvalue_8 (Math|Float|Clamp(Float) _returnvalue_7 0.0 _returnvalue_2))
  (Transformation|SetWorldRotation (Variables|Default|GetBoutonGauche) (Math|Rotator|MakeRotator 0.0 _returnvalue_8 0.0) false false)
  (bind _output_get (Variables|Default|SetGetRotationYRight _returnvalue_8))
  (Default|ChangeValue (Variables|Default|GetCanonView) (/ (stale Custom|TickLeft _output_get) 1.8e+02) (/ _output_get 1.8e+02))
  (Variables|/Game/Game/Blueprints/Cannon/BP_Scaner.BP_Scaner_C|SetBAngle _scaner (- (* (/ _output_get 1.8e+02) 3.6e+02) 1.8e+02))
  (bind _result (Math|Float|NegateFloat (- (* (/ (stale Custom|TickLeft _output_get) 1.8e+02) 3.6e+02) 1.8e+02))
    (:%20%20
      (Variables|/Game/Game/Blueprints/Cannon/BP_Scaner.BP_Scaner_C|SetAAngle _scaner _result))))

(event EventBeginPlay
  (bind _aswbp_canon_view (Utilities|Casting|CastToWBP_CanonView (UserInterface|GetWidget (Variables|Default|GetTargetHUD))))
  (Variables|Default|SetCanonView _aswbp_canon_view)
  (bind _aswbp_monster_view (Utilities|Casting|CastToWBP_MonsterView (UserInterface|GetWidget (Variables|Default|GetMonsterHUD))))
  (Variables|Default|SetMonsterView _aswbp_monster_view))

(event EventDeinteract
  (Collision|SetCollisionEnabled (Variables|Default|Get%20) "NoCollision")
  (Utilities|Time|PauseTimerbyHandle (Variables|Default|GetUnset))
  (Variables|Default|SetRotationYRight (Variables|Default|GetGetRotationYRight))
  (Variables|Default|SetRotationYLeft (Variables|Default|GetGetRotationYLeft)))

(event EventInteract
  (params (PlayerRef :type BP%20First%20Person%20Character%20Object%20Reference))
  (bind _arrow (Variables|Default|GetArrow))
  ;[0.15 0.15 0.15 0.5] Caméra sur moniteur
  (Default|TeleportCamera PlayerRef (Math|Transform|MakeTransform (Transformation|GetWorldLocation _arrow) (Transformation|GetWorldRotation _arrow) "1.000000,1.000000,1.000000"))
  (Collision|SetCollisionEnabled (Variables|Default|Get%20) "QueryAndPhysics"))

(fn ConstructionScript)