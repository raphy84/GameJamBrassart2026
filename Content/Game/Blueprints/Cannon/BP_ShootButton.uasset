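; Cannon button that alternates between starting a charge and firing through a FlipFlop, after an animated press guarded by a re-press lock.
; A fast looping timer raises the charge, updating the WBP_ChargeCanon display and sound pitch, and fires automatically at maximum.
; Firing passes the charge to ScanerRef.Shoot with sound and camera shake, then a delayed second timer drains the charge with a falling pitch.
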(event Custom|CustomEvent
  (bind _result (Math|Float|DecrementFloat (Variables|Default|GetPoint))
    (:%20%20
      (Default|SetME (Variables|Default|GetWidgetChargeCanon) (Variables|Default|GetPoint))
      (Audio|Components|Audio|SetPitchMultiplier (stale Custom|Tick _returnvalue_4) (Math|Float|Lerp 0.0 1.0 (Math|Float|MapRangeClamped _result 8e+04 0.0 1.0 0.0)))
      (if (>= 0.0 (Variables|Default|GetPoint))
        (Utilities|Time|PauseTimerbyHandle (Variables|Default|GetTimer))
        (Audio|Components|Audio|Stop (stale Custom|Tick _returnvalue_4))))))

(event Custom|Tick
  (bind _result (Math|Float|IncrementFloat (Variables|Default|GetPoint))
    (:%20%20
      (Default|SetME (Variables|Default|GetWidgetChargeCanon) (Variables|Default|GetPoint))
      (Variables|Default|SetIsCharging true)
      (Audio|Components|Audio|SetPitchMultiplier (stale _returnvalue) (Math|Float|Lerp 0.0 1.0 (Math|Float|MapRangeClamped _result 0.0 8e+04 0.0 1.0)))
      (if (>= (Variables|Default|GetPoint) 8e+04)
        (Utilities|FlowControl|FlipFlop
          (:A
            (Utilities|IsValid (stale _returnvalue_4)
              (:Is%20Valid
                (Audio|Components|Audio|Stop (stale _returnvalue_4)))
              (:Is%20Not%20Valid
                _))
            (bind _returnvalue (Audio|SpawnSound2D "/Game/Game/SoundDesign/Recharge.Recharge" 0.1 0.0 0.0 0))
            (Utilities|Time|PauseTimerbyHandle (Variables|Default|GetTimer))
            (bind _returnvalue_2 (Utilities|Time|SetTimerbyEvent (delegate Custom|Tick) 0.0001 true))
            (Variables|Default|SetTimer _returnvalue_2))
          (:B
            (Utilities|Time|PauseTimerbyHandle (Variables|Default|GetTimer))
            (Default|Shoot (Variables|Default|GetScanerRef) (Variables|Default|GetPoint))
            (Variables|Default|SetDelay false)
            (Utilities|FlowControl|Sequence
              (:then_0
                (Utilities|FlowControl|Delay 0.3)
                (Audio|Components|Audio|Stop _returnvalue)
                (Utilities|FlowControl|Delay 2.0)
                (bind _returnvalue_3 (Utilities|Time|SetTimerbyEvent (delegate Custom|CustomEvent) 0.0001 true))
                (Variables|Default|SetTimer _returnvalue_3)
                (Variables|Default|SetDelay true)
                (bind _returnvalue_4 (Audio|SpawnSound2D "/Game/Game/SoundDesign/BaisseRecharge_Cue.BaisseRecharge_Cue" 1.0 0.0 0.0 0)))
              (:then_1
                (Audio|SpawnSound2D "/Game/Game/SoundDesign/Tir_Cue.Tir_Cue" 0.45 1.0 0.0 0)
                (Camera|PlayWorldCameraShake "/Game/Game/Blueprints/Cannon/BP_ShakeScreen.BP_ShakeScreen_C" "0, 0, 0" 0.0 2e+03 2.0 true)))))))))

(event EventBeginPlay
  (bind _aswbp_charge_canon (Utilities|Casting|CastToWBP_ChargeCanon (UserInterface|GetWidget (Variables|Default|GetWidgetCanon))))
  (Variables|Default|SetWidgetChargeCanon _aswbp_charge_canon))

(event EventPress
  (bind _buttonmid (Variables|Default|GetButtonMid))
  (bind _relativelocation (Variables|/Script/Engine.SceneComponent|GetRelativeLocation _buttonmid))
  (if (Variables|Default|GetDelay)
    (Audio|SpawnSound2D "/Game/Game/SoundDesign/BtnPress.BtnPress" 1.2 1.0 0.2 0)
    (Variables|Default|SetDelay false)
    (bind _buttonanim (Timeline|Timeline PlayFromStart)
      (:Update
        (bind _result (Math|Float|NegateFloat _buttonanim)
          (:%20%20
            (Transformation|SetRelativeLocation _buttonmid (Math|Vector|MakeVector (.x _relativelocation) (.y _relativelocation) _result) false false))))
      (:Finished
        (Variables|Default|SetDelay true)
        (Utilities|FlowControl|FlipFlop
          (:A
            (Utilities|IsValid (stale _returnvalue_4)
              (:Is%20Valid
                (Audio|Components|Audio|Stop (stale _returnvalue_4)))
              (:Is%20Not%20Valid
                _))
            (bind _returnvalue (Audio|SpawnSound2D "/Game/Game/SoundDesign/Recharge.Recharge" 0.1 0.0 0.0 0))
            (Utilities|Time|PauseTimerbyHandle (Variables|Default|GetTimer))
            (bind _returnvalue_2 (Utilities|Time|SetTimerbyEvent (delegate Custom|Tick) 0.0001 true))
            (Variables|Default|SetTimer _returnvalue_2))
          (:B
            (Utilities|Time|PauseTimerbyHandle (Variables|Default|GetTimer))
            (Default|Shoot (Variables|Default|GetScanerRef) (Variables|Default|GetPoint))
            (Variables|Default|SetDelay false)
            (Utilities|FlowControl|Sequence
              (:then_0
                (Utilities|FlowControl|Delay 0.3)
                (Audio|Components|Audio|Stop _returnvalue)
                (Utilities|FlowControl|Delay 2.0)
                (bind _returnvalue_3 (Utilities|Time|SetTimerbyEvent (delegate Custom|CustomEvent) 0.0001 true))
                (Variables|Default|SetTimer _returnvalue_3)
                (Variables|Default|SetDelay true)
                (bind _returnvalue_4 (Audio|SpawnSound2D "/Game/Game/SoundDesign/BaisseRecharge_Cue.BaisseRecharge_Cue" 1.0 0.0 0.0 0)))
              (:then_1
                (Audio|SpawnSound2D "/Game/Game/SoundDesign/Tir_Cue.Tir_Cue" 0.45 1.0 0.0 0)
                (Camera|PlayWorldCameraShake "/Game/Game/Blueprints/Cannon/BP_ShakeScreen.BP_ShakeScreen_C" "0, 0, 0" 0.0 2e+03 2.0 true)))))))))

(fn ConstructionScript)