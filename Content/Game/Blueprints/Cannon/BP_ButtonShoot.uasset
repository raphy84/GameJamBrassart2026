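; Interactable cannon button that charges a shot and scares off monsters whose hated frequency matches the charge.
; Interact alternates between starting a looping timer that raises CannonCharge and pausing it to fire, with automatic firing at a cap.
; Shoot calls Running on tracked monsters with FrequenceHate near the charge, but zeroes the charge inside the loop after the first check.
; SuperFonction adds or removes monsters as their range state changes.
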(event Custom|Tick
  (bind _output_get (Variables|Default|SetCannonCharge (+ (Variables|Default|GetCannonCharge) 1)))
  (Development|PrintString (Utilities|String|ToString(Integer) _output_get))
  (if (== (Variables|Default|GetCannonCharge) 500)
    (Utilities|Time|PauseTimerbyHandle (stale EventInteract _returnvalue))
    (CallFunction|Shoot)))

(event Custom|Shoot
  (bind _monstre (Variables|Default|GetMonstre))
  (Development|PrintString (Utilities|String|ToString(Integer) (Utilities|Array|Length _monstre)))
  (for _array_element _monstre
    (Development|PrintString (Utilities|String|ToString(Integer) (Variables|/Game/Game/Blueprints/IA/BP_Monster.BP_Monster_C|GetFrequenceHate _array_element)) true true "(R=0.059086,G=1.000000,B=0.000000,A=1.000000)")
    (if (Math|Float|InRange(Float) (Math|Conversions|ToFloat(Integer) (Variables|/Game/Game/Blueprints/IA/BP_Monster.BP_Monster_C|GetFrequenceHate _array_element)) (Math|Conversions|ToFloat(Integer) (- (Variables|Default|GetCannonCharge) 50)) (Math|Conversions|ToFloat(Integer) (+ (Variables|Default|GetCannonCharge) 50)))
      (Variables|Default|SetCannonCharge 0)
      (Default|Running _array_element)
      (else
        (Variables|Default|SetCannonCharge 0)))))

(event EventBeginPlay)

(event Collision|EventActorBeginOverlap
  (params (OtherActor :type Actor%20Object%20Reference)))

(event EventTick
  (params (DeltaSeconds :type Float%20%28single-precision%29)))

(event EventInteract
  (params (PlayerRef :type BP%20First%20Person%20Character%20Object%20Reference))
  (Utilities|FlowControl|FlipFlop
    (:A
      (bind _returnvalue (Utilities|Time|SetTimerbyEvent (delegate Custom|Tick) 0.01 true)))
    (:B
      (Utilities|Time|PauseTimerbyHandle _returnvalue)
      (CallFunction|Shoot))))

(event EventSuperFonction
  (params (IsInRange :type Boolean) (NewParam :type BP%20Monster%20Object%20Reference))
  (if IsInRange
    (Utilities|Array|AddUnique (Variables|Default|GetMonstre) NewParam)
    (else
      (Utilities|Array|RemoveItem (Variables|Default|GetMonstre) NewParam))))

(fn ConstructionScript)