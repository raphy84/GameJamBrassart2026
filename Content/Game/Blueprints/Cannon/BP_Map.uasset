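; Interactable map console for aiming the cannon: interacting teleports the player's camera to it and enables a collider.
; Clicking either knob starts a fast looping timer that turns horizontal mouse drag into clamped rotation; release pauses it and saves the angle.
; One knob sets angle, the other range, updating WBP_Map and calling AimCanon on the scanner.
; Knobs play click sounds, with DoOnce gates tracking range steps.
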(event OnClicked(BoutonGauche)
  (params (TouchedComponent :type Primitive%20Component%20Object%20Reference) (ButtonPressed :type Key%20Structure :default "None"))
  (Variables|Default|SetLocationX (.LocationX (Game|Player|GetMousePosition (Game|GetPlayerController 0))))
  (bind _returnvalue (Utilities|Time|SetTimerbyEvent (delegate Custom|Tick) 0.001 true))
  (Variables|Default|SetUnset _returnvalue))

(event OnReleased(BoutonGauche)
  (params (TouchedComponent :type Primitive%20Component%20Object%20Reference) (ButtonReleased :type Key%20Structure :default "None"))
  (Utilities|Time|PauseTimerbyHandle (Variables|Default|GetUnset))
  (Variables|Default|SetRotationYRight (Variables|Default|GetGetRotationYRight))
  (Variables|Default|SetRotationYLeft (Variables|Default|GetGetRotationYLeft)))

(event OnReleased(0)
  (params (TouchedComponent :type Primitive%20Component%20Object%20Reference) (ButtonReleased :type Key%20Structure :default "None"))
  (Utilities|Time|PauseTimerbyHandle (Variables|Default|GetUnset))
  (Variables|Default|SetRotationYRight (Variables|Default|GetGetRotationYRight))
  (Variables|Default|SetRotationYLeft (Variables|Default|GetGetRotationYLeft)))

(event OnClicked(BoutonGauche1)
  (params (TouchedComponent :type Primitive%20Component%20Object%20Reference) (ButtonPressed :type Key%20Structure :default "None"))
  (Variables|Default|SetLocationX (.LocationX (Game|Player|GetMousePosition (Game|GetPlayerController 0))))
  (bind _returnvalue (Utilities|Time|SetTimerbyEvent (delegate Custom|Tick2) 0.001 true))
  (Variables|Default|SetUnset _returnvalue))

(event OnReleased(BoutonGauche1)
  (params (TouchedComponent :type Primitive%20Component%20Object%20Reference) (ButtonReleased :type Key%20Structure :default "None"))
  (Utilities|Time|PauseTimerbyHandle (Variables|Default|GetUnset))
  (Variables|Default|SetRotationYRight (Variables|Default|GetGetRotationYRight))
  (Variables|Default|SetRotationYLeft (Variables|Default|GetGetRotationYLeft)))

(event Custom|Tick
  (bind _returnvalue (Game|GetPlayerController 0))
  (bind _locationx (Variables|Default|GetLocationX))
  (bind _rotationyright (Variables|Default|GetRotationYRight))
  (bind _boutongauche (Variables|Default|GetBoutonGauche))
  (bind _locationx_2 (Game|Player|GetMousePosition _returnvalue))
  (bind _returnvalue_2 (Transformation|GetWorldRotation _boutongauche))
  (bind _returnvalue_3 (- _locationx _locationx_2))
  (bind _returnvalue_4 (/ _returnvalue_3 3.0))
  (bind _returnvalue_5 (+ _rotationyright _returnvalue_4))
  (bind _returnvalue_6 (Math|Float|NormalizetoRange _returnvalue_5 0.0 1.8e+02))
  (bind _returnvalue_7 (+ _returnvalue_5 _returnvalue_6))
  (bind _returnvalue_8 (Math|Float|Clamp(Float) _returnvalue_7 0.0 9e+01))
  (Transformation|SetWorldRotation _boutongauche (Math|Rotator|MakeRotator (.roll _returnvalue_2) _returnvalue_8 (.yaw _returnvalue_2)) false false)
  (bind _output_get (Variables|Default|SetGetRotationYRight _returnvalue_8))
  (bind _result (Math|Float|NegateFloat (* (/ _output_get 9e+01) 7.0))
    (:%20%20
      (Default|MoveVisual (Variables|Default|GetWidgetMap) _result)
      (Utilities|FlowControl|Sequence
        (:then_0
          (Default|AimCanon (Variables|Default|GetScanerRef) (Math|Float|MapRangeClamped _output_get 9e+01 0.0 135.0 -1.8e+02) (* (/ (stale Custom|Tick2 _output_get) 9e+01) 4.0)))
        (:then_1
          (if (!= (Variables|Default|GetValueTest) (Variables|Default|GetGetRotationYRight))
            (Variables|Default|SetValueTest (Variables|Default|GetGetRotationYRight))
            (Utilities|FlowControl|Delay 0.05)
            (bind _returnvalue_9 (Audio|SpawnSound2D "/Game/Game/SoundDesign/CrickBtn_Cue.CrickBtn_Cue" 0.1 1.0 0.0 0))
            (else
              (Utilities|IsValid _returnvalue_9
                (:Is%20Valid
                  (Components|DestroyComponent _returnvalue_9))))))))))

(event Custom|Tick2
  (bind _returnvalue (Game|GetPlayerController 0))
  (bind _locationx (Variables|Default|GetLocationX))
  (bind _boutongauche1 (Variables|Default|GetBoutonGauche1))
  (bind _rotationyleft (Variables|Default|GetRotationYLeft))
  (bind _returnvalue_2 (Transformation|GetWorldRotation _boutongauche1))
  (bind _locationx_2 (Game|Player|GetMousePosition _returnvalue))
  (bind _returnvalue_3 (- _locationx _locationx_2))
  (bind _returnvalue_4 (/ _returnvalue_3 3.0))
  (bind _returnvalue_5 (+ _rotationyleft _returnvalue_4))
  (bind _returnvalue_6 (Math|Float|NormalizetoRange _returnvalue_5 0.0 1.8e+02))
  (bind _returnvalue_7 (+ _returnvalue_5 _returnvalue_6))
  (bind _returnvalue_8 (Math|Float|Clamp(Float) _returnvalue_7 0.0 9e+01))
  (Transformation|SetWorldRotation _boutongauche1 (Math|Rotator|MakeRotator (.roll _returnvalue_2) _returnvalue_8 (.yaw _returnvalue_2)) false false)
  (bind _output_get (Variables|Default|SetGetRotationYLeft _returnvalue_8))
  (Default|MoveRange (Variables|Default|GetWidgetMap) (* (/ _output_get 9e+01) 4.0))
  (Utilities|FlowControl|Sequence
    (:then_0
      (Default|AimCanon (Variables|Default|GetScanerRef) (Math|Float|MapRangeClamped (stale Custom|Tick _output_get) 9e+01 0.0 135.0 -1.8e+02) (* (/ _output_get 9e+01) 4.0)))
    (:then_1
      (if (!= (Variables|Default|GetValueTest) (Variables|Default|GetGetRotationYLeft))
        (Variables|Default|SetValueTest (Variables|Default|GetGetRotationYLeft))
        (switch int (Math|Float|Truncate (* (/ _output_get 9e+01) 4.0))
          (:0
            (Utilities|FlowControl|Sequence
              (:then_0
                (Utilities|FlowControl|DoOnce false :!label _label
                  (:Completed
                    _)))
              (:then_1
                (goto _label_2 Reset))
              (:then_2
                (goto _label_3 Reset))
              (:then_3
                (goto _label_4 Reset))
              (:then_4
                (goto _label_5 Reset))))
          (:1
            (Utilities|FlowControl|Sequence
              (:then_0
                (goto _label Reset))
              (:then_1
                (Utilities|FlowControl|DoOnce false :!label _label_2
                  (:Completed
                    _)))
              (:then_2
                (goto _label_3 Reset))
              (:then_3
                (goto _label_4 Reset))
              (:then_4
                (goto _label_5 Reset))))
          (:2
            (Utilities|FlowControl|Sequence
              (:then_0
                (goto _label Reset))
              (:then_1
                (goto _label_2 Reset))
              (:then_2
                (Utilities|FlowControl|DoOnce false :!label _label_3
                  (:Completed
                    _)))
              (:then_3
                (goto _label_4 Reset))
              (:then_4
                (goto _label_5 Reset))))
          (:3
            (Utilities|FlowControl|Sequence
              (:then_0
                (goto _label Reset))
              (:then_1
                (goto _label_2 Reset))
              (:then_2
                (goto _label_3 Reset))
              (:then_3
                (Utilities|FlowControl|DoOnce false :!label _label_4
                  (:Completed
                    _)))
              (:then_4
                (goto _label_5 Reset))))
          (:4
            (Utilities|FlowControl|Sequence
              (:then_0
                (goto _label Reset))
              (:then_1
                (goto _label_2 Reset))
              (:then_2
                (goto _label_3 Reset))
              (:then_3
                (goto _label_4 Reset))
              (:then_4
                (Utilities|FlowControl|DoOnce false :!label _label_5
                  (:Completed
                    _))))))
        (bind _returnvalue_9 (Audio|SpawnSound2D "/Game/Game/SoundDesign/CrickBtn_Cue.CrickBtn_Cue" 0.1 1.0 0.0 0))
        (else
          (Utilities|IsValid _returnvalue_9
            (:Is%20Valid
              (Components|DestroyComponent _returnvalue_9))))))))

(event EventBeginPlay
  (bind _aswbp_map (Utilities|Casting|CastToWBP_Map (UserInterface|GetWidget (Variables|Default|GetMonsterHUD))))
  (Variables|Default|SetWidgetMap _aswbp_map))

(event EventInteract
  (params (PlayerRef :type BP%20First%20Person%20Character%20Object%20Reference))
  (Default|TeleportCamera PlayerRef (Transformation|GetWorldTransform (Variables|Default|GetArrow)))
  (Collision|SetCollisionEnabled (Variables|Default|Get0) "QueryAndPhysics"))

(event EventDeinteract
  (Utilities|Time|PauseTimerbyHandle (Variables|Default|GetUnset))
  (Variables|Default|SetRotationYRight (Variables|Default|GetGetRotationYRight))
  (Variables|Default|SetRotationYLeft (Variables|Default|GetGetRotationYLeft))
  (Collision|SetCollisionEnabled (Variables|Default|Get0) "NoCollision"))

(fn ConstructionScript)