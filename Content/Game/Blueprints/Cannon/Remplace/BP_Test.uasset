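; Test actor that checks whether BP_Monster actors fall inside an adjustable slice of a circle and reports each result to BP_ButtonShoot.
; O/P and L/M keys move two percentage-based arrows, which Tick clamps and converts to circle points.
; Each monster is tested against the centre-and-arrows triangle by comparing sub-triangle areas, with debug lines and prints.
; The area formula repeats a Y term, and the computed segment area is unused.
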(event EventBeginPlay)

(event Collision|EventActorBeginOverlap
  (params (OtherActor :type Actor%20Object%20Reference)))

(event EventTick
  (params (DeltaSeconds :type Float%20%28single-precision%29))
  (Variables|Default|SetArrow1Position (Math|Float|Clamp(Float) (Variables|Default|GetArrow1Position) 0.01 (- (Variables|Default|GetArrow2Position) 1.0)))
  (Variables|Default|SetArrow2Position (Math|Float|Clamp(Float) (Variables|Default|GetArrow2Position) (+ (Variables|Default|GetArrow1Position) 1.0) 1e+02))
  (bind _worldposition (CallFunction|GetPointonCircle self (Variables|Default|GetArrow1Position)))
  (Variables|Default|SetPoint1 _worldposition)
  (bind _worldposition_2 (CallFunction|GetPointonCircle self (Variables|Default|GetArrow2Position)))
  (Variables|Default|SetPoint2 _worldposition_2)
  (CallFunction|CalculateSegmentArea self)
  (bind _outactors (Actor|GetAllActorsOfClass "/Game/Game/Blueprints/IA/BP_Monster.BP_Monster_C"))
  (for _array_element _outactors
    (bind _is_in_segment (CallFunction|IsMonsterinSegment self (Transformation|GetActorLocation _array_element)))
    (bind _returnvalue (Actor|GetActorOfClass "/Game/Game/Blueprints/Cannon/BP_ButtonShoot.BP_ButtonShoot_C"))
    (Default|SuperFonction _returnvalue _is_in_segment _array_element)))

(event Input|KeyboardEvents|O
  (params (Key :type Key%20Structure :default "None"))
  (:Pressed
    (Variables|Default|SetArrow1Position (+ (Variables|Default|GetArrow1Position) 5.0))))

(event Input|KeyboardEvents|P
  (params (Key :type Key%20Structure :default "None"))
  (:Pressed
    (Variables|Default|SetArrow1Position (- (Variables|Default|GetArrow1Position) 5.0))))

(event Input|KeyboardEvents|L
  (params (Key :type Key%20Structure :default "None"))
  (:Pressed
    (Variables|Default|SetArrow2Position (+ (Variables|Default|GetArrow2Position) 5.0))))

(event Input|KeyboardEvents|M
  (params (Key :type Key%20Structure :default "None"))
  (:Pressed
    (Variables|Default|SetArrow2Position (- (Variables|Default|GetArrow2Position) 5.0))))

(fn ConstructionScript)

(fn SetArrow1Position
  (params (NewPosition :type Float%20%28double-precision%29))
  (Variables|Default|SetArrow1Position (Math|Float|Clamp(Float) NewPosition 0.01 (- (Variables|Default|GetArrow2Position) 1.0))))

(fn SetArrow2Position
  (params (NewPosition :type Float%20%28double-precision%29))
  (Variables|Default|SetArrow2Position (Math|Float|Clamp(Float) NewPosition (+ (Variables|Default|GetArrow1Position) 1.0) 1e+02)))

(fn GetPointonCircle
  (params (ArrowValue :type Float%20%28double-precision%29))
  (bind _returnvalue (/ ArrowValue 1e+02))
  (bind _radius (Variables|Default|GetRadius))
  (bind _returnvalue_2 (* _returnvalue 3.6e+02))
  (bind _returnvalue_3 (Math|Trig|DegreesToRadians _returnvalue_2))
  (return (+ (Math|Vector|MakeVector (* (Math|Trig|Cos(Radians) _returnvalue_3) _radius) (* (Math|Trig|Sin(Radians) _returnvalue_3) _radius) 0.0) (Variables|Default|GetCenterPoint))))

(fn CalculateSegmentArea
  (bind _radius (Variables|Default|GetRadius))
  (LocalVariables|SetThetaRandians (* (/ (- (Variables|Default|GetArrow2Position) (Variables|Default|GetArrow1Position)) 1e+02) 6.28318))
  (return (* (/ (* _radius _radius) 2.0) (- (LocalVariables|GetThetaRandians) (Math|Trig|Sin(Radians) (LocalVariables|GetThetaRandians))))))

(fn IsMonsterinSegment
  (params (MonsterLocation :type Vector))
  (LocalVariables|SetPM MonsterLocation)
  (LocalVariables|SetP0 (Variables|Default|GetCenterPoint))
  (bind _worldposition (CallFunction|GetPointonCircle (Variables|Default|GetArrow1Position)))
  (LocalVariables|SetP1 _worldposition)
  (bind _worldposition_2 (CallFunction|GetPointonCircle (Variables|Default|GetArrow2Position)))
  (LocalVariables|SetP2 _worldposition_2)
  (Rendering|Debug|DrawDebugLine (LocalVariables|GetP0) (LocalVariables|GetP1) "(R=0.000000,G=1.000000,B=0.000000,A=1.000000)" 0.1 2.0)
  (Rendering|Debug|DrawDebugLine (LocalVariables|GetP1) (LocalVariables|GetP2) "(R=1.000000,G=0.000000,B=0.000000,A=1.000000)" 0.1 2.0)
  (Rendering|Debug|DrawDebugLine (LocalVariables|GetP2) (LocalVariables|GetP0) "(R=0.000000,G=0.000000,B=1.000000,A=1.000000)" 0.1 2.0)
  (bind _area (CallFunction|CalculateTriangle (LocalVariables|GetP0) (LocalVariables|GetP1) (LocalVariables|GetP2)))
  (bind _area_2 (CallFunction|CalculateTriangle (LocalVariables|GetPM) (LocalVariables|GetP1) (LocalVariables|GetP2)))
  (bind _area_3 (CallFunction|CalculateTriangle (LocalVariables|GetP0) (LocalVariables|GetPM) (LocalVariables|GetP2)))
  (bind _area_4 (CallFunction|CalculateTriangle (LocalVariables|GetP0) (LocalVariables|GetP1) (LocalVariables|GetPM)))
  (Development|PrintString (Utilities|String|ToString(Boolean) (< (- (+ _area_2 _area_3 _area_4) _area) 0.01)))
  (return (< (- (+ _area_2 _area_3 _area_4) _area) 0.01)))

(fn CalculateTriangle
  (params (Point1 :type Vector) (Point2 :type Vector) (Point3 :type Vector))
  (bind (_x _y) (Math|Vector|BreakVector Point1))
  (bind (_x_2 _y_2) (Math|Vector|BreakVector Point3))
  (return (/ (Math|Float|Absolute(Float) (- (* (- _x _x_2) (- _y _y_2)) (* (- (.X (Math|Vector|BreakVector Point2)) _x_2) (- _y _y_2)))) 2.0)))