(event EventTick
  (params (DeltaSeconds :type Float%20%28single-precision%29)))

(event EventSuperFonction
  (params (IsInRange :type Boolean) (NewParam :type BP%20Monster%20Object%20Reference))
  (Variables|Default|SetTestPoint "0, 0, 0"))

(fn ConstructionScript)