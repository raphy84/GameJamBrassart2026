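; BP_Codex is an interactable codex actor that shows a localized page on a plane and moves the player's camera to view it.
; On BeginPlay it reads BP_GameInstance, hiding itself in duo mode and choosing the FR or AN plane material from FRMode.
; Interact calls TeleportCamera on the player using the Arrow component's world transform as the viewpoint.
; The construction script previews the French material.
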(event EventBeginPlay
  (bind _asbp_game_instance (Utilities|Casting|CastToBP_GameInstance (Game|GetGameInstance)))
  (Utilities|FlowControl|Sequence
    (:then_0
      (if (Variables|/Game/Game/Blueprints/BP_GameInstance.BP_GameInstance_C|GetDuoMode _asbp_game_instance)
        (Rendering|SetActorHiddenInGame true)
        (else
          (Rendering|SetActorHiddenInGame false))))
    (:then_1
      (if (Variables|/Game/Game/Blueprints/BP_GameInstance.BP_GameInstance_C|GetFRMode _asbp_game_instance)
        (Rendering|Material|SetMaterial (Variables|Default|GetPlane) 0 (Variables|Default|GetMaterialFR))
        (else
          (Rendering|Material|SetMaterial (Variables|Default|GetPlane) 0 (Variables|Default|GetMaterialAN)))))))

(event EventInteract
  (params (PlayerRef :type BP%20First%20Person%20Character%20Object%20Reference))
  (bind _arrow (Variables|Default|GetArrow))
  (Default|TeleportCamera PlayerRef (Math|Transform|MakeTransform (Transformation|GetWorldLocation _arrow) (Transformation|GetWorldRotation _arrow) "1.000000,1.000000,1.000000")))

(fn ConstructionScript
  (Rendering|Material|SetMaterial (Variables|Default|GetPlane) 0 (Variables|Default|GetMaterialFR)))