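; Monster spawner that runs day-based waves, starting with one delayed monster from the first array entry at BeginPlay.
; A looping timer checks for any living BP_Monster; when none remains, it increments Day, updates DayNum and spawns Day minus one random monsters.
; Each spawn follows a random actor yaw, swinging SpawnPoint to a new spot.
; Wave monsters get random start delays whose upper limit grows with Day.
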(event Custom|CanSpawn
  (bind _returnvalue (Actor|GetActorOfClass "/Game/Game/Blueprints/IA/BP_Monster.BP_Monster_C"))
  (Utilities|IsValid _returnvalue
    (:Is%20Not%20Valid
      (bind _result (Math|Integer|IncrementInt (Variables|Default|GetDay))
        (:%20%20
          (Default|SetData (Variables|Default|GetDayNum) _result)
          (Variables|Default|SetNum (- (Variables|Default|GetDay) 1))
          (if (> (Variables|Default|GetNum) 0) :!label _label
            (Transformation|SetActorRotation (Math|Rotator|MakeRotator 0.0 0.0 (Math|Random|RandomFloatinRange -1.8e+02 1.8e+02)))
            (bind _returnvalue_2 (Game|SpawnActorfromClass (.OutItem (Utilities|Array|Random (Variables|Default|GetMonsterArray))) (Transformation|GetWorldTransform (Variables|Default|GetSpawnPoint)) "AlwaysSpawn" "MultiplyWithRoot" 0 0))
            (Variables|/Game/Game/Blueprints/IA/BP_Monster.BP_Monster_C|SetDelayStart _returnvalue_2 (Math|Random|RandomFloatinRange 0.0 (* 3e+01 (Variables|Default|GetDay))))
            (Math|Integer|DecrementInt (Variables|Default|GetNum)
              (:%20%20
                (goto _label)))))))))

(event EventBeginPlay
  (Transformation|SetActorRotation (Math|Rotator|MakeRotator 0.0 0.0 (Math|Random|RandomFloatinRange -1.8e+02 1.8e+02)))
  (bind _returnvalue (Game|SpawnActorfromClass (Utilities|Array|Get(acopy) (Variables|Default|GetMonsterArray)) (Transformation|GetWorldTransform (Variables|Default|GetSpawnPoint)) "AlwaysSpawn" "MultiplyWithRoot" 0 0))
  (Variables|/Game/Game/Blueprints/IA/BP_Monster.BP_Monster_C|SetDelayStart _returnvalue 3e+01)
  (Utilities|Time|SetTimerbyEvent (delegate Custom|CanSpawn) 1e+01 true))

(fn ConstructionScript)