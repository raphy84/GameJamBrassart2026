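; BP_Monster is a monster that, after a start delay, creeps from its spawn point toward a player location set to the world origin by advancing a Lerp alpha every tick.
; A looping timer plays distance-scaled impact sounds and camera shakes during the approach.
; TryRun checks a frequency against the monster's hated range; a match reverses its speed, plays a sound and shake, and lets it destroy itself back at spawn.
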(event Custom|Boom
  (bind _returnvalue (Transformation|GetActorLocation))
  (Audio|SpawnSoundatLocation "/Game/Game/SoundDesign/Impact.Impact" _returnvalue "0, 0, 0" (Math|Float|MapRangeClamped (Math|Vector|Distance(Vector) (Transformation|GetActorLocation) (Variables|Default|GetPlayerLocation)) 1.5e+03 0.0 0.0 0.7) 0.01 0.0 0 0)
  (Utilities|FlowControl|Delay 0.5)
  (Camera|PlayWorldCameraShake "/Game/Game/Blueprints/Cannon/BP_ShakeScreen.BP_ShakeScreen_C" _returnvalue 0.0 2e+03 3.0 true))

(event EventBeginPlay
  (Variables|Default|SetMonsterSpawn (Transformation|GetActorLocation))
  (Variables|Default|SetPlayerLocation "0, 0, 0")
  (Utilities|FlowControl|Delay 1.0)
  (Utilities|FlowControl|Delay (Variables|Default|GetDelayStart))
  (Variables|Default|SetActivate true)
  (Utilities|Time|SetTimerbyEvent (delegate Custom|Boom) 2.0 true))

(event EventTryRun
  (params (Frequence :type Float%20%28double-precision%29))
  (if (and (<= Frequence (Variables|Default|GetFrequenceHateUp)) (>= Frequence (Variables|Default|GetFrequenceHateDown)))
    (Variables|Default|SetRunLocation (Transformation|GetActorLocation))
    (Variables|Default|SetSpeed -0.0005)
    (Variables|Default|SetCanDie true)
    (Utilities|FlowControl|Delay 0.5)
    (Audio|PlaySound2D "/Game/Game/SoundDesign/PasContent_Cue.PasContent_Cue" 0.2 1.0 0.0 0 0)
    (Camera|PlayWorldCameraShake "/Game/Game/Blueprints/Cannon/BP_ShakeScreen.BP_ShakeScreen_C" "0, 0, 0" 0.0 2e+03 1e+01)))

(event EventTick
  (params (DeltaSeconds :type Float%20%28single-precision%29))
  (if (Variables|Default|GetActivate)
    (bind _output_get (Variables|Default|SetLocation (+ (Variables|Default|GetSpeed) (Variables|Default|GetLocation))))
    (Transformation|SetActorLocation (Math|Vector|Lerp(Vector) (Variables|Default|GetMonsterSpawn) (Variables|Default|GetPlayerLocation) _output_get) true false)
    (if (Variables|Default|GetCanDie)
      (if (Utilities|Operators|EqualEqual (Transformation|GetActorLocation) (Variables|Default|GetMonsterSpawn) 1.0)
        (Actor|DestroyActor)))))

(fn ConstructionScript)